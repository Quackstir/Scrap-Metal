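; BP_S_Movement is an entity stat Blueprint that modifies an entity's movement speed.
; On initialization it runs the parent setup and caches the entity's BPMovementStatComponent.
; Updates pass that component's BaseMovementSpeed to the parent calculation as the initial value, overriding the caller's initial-value inputs.
; The result is printed and then applied through the component's ModifyMovement.
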(event EventInitializeStat
  (params (Entity :type BP%20Entity%20Base%20Object%20Reference) (Struct%20Stats :type Struct%20Stat%20Structure))
  (|CallParentFunction Entity Struct%20Stats)
  (Variables|Default|SetBP%20Movement%20Stat%20Component (Variables|/Game/Blueprints/Entities/BP_EntityBase_Auto2.BP_EntityBase_C|GetBP_MovementStatComponent (Variables|Default|GetEntity))))

(fn UpdateStat
  (params (Amount :type Integer) (Using%20Initial%20Val%20Struct :type Boolean) (New%20Initial%20Val :type Float%20%28double-precision%29))
  (bind _bp_movement_stat_component (Variables|Default|GetBP%20Movement%20Stat%20Component))
  (bind _progression_value (|CallParentFunction Amount false (Variables|/Game/Blueprints/Entities/EntityComponents/BP_MovementStatComponent.BP_MovementStatComponent_C|GetBase%20MovementSpeed _bp_movement_stat_component)))
  (Development|PrintString (Utilities|String|ToString(Float) _progression_value))
  (Default|ModifyMovement _bp_movement_stat_component _progression_value))