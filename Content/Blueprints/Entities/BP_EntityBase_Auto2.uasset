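; BP_EntityBase_Auto2 is an entity base Blueprint that initializes health, movement and mod manager components on BeginPlay.
; Event dispatchers announce item use, special movement and shield recharge, while the damage dispatch is unreachable.
; Primary input fires item use directly, bypassing the CanUsePrimary check in PrimaryAction, and debug-style keys adjust health.
; Shield and damage stats live on the entity, but their initializers are not called here.
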(event EventBeginPlay
  (CallFunction|InitializeStats))

(event Input|ActionEvents|InputActionPrimaryAction
  (params (Key :type Key%20Structure :default "None"))
  (:Pressed
    (Default|CallOnUseItem)))

(event Input|KeyboardEvents|Subtract
  (params (Key :type Key%20Structure :default "None"))
  (bind _bp_healthcomponent (Variables|Default|GetBP_HealthComponent))
  (:Pressed
    (Default|SetHealth _bp_healthcomponent (- (Variables|/Game/Blueprints/Entities/EntityComponents/BP_HealthComponent.BP_HealthComponent_C|GetCurr%20Health _bp_healthcomponent) 10))))

(event Input|KeyboardEvents|Add
  (params (Key :type Key%20Structure :default "None"))
  (bind _bp_healthcomponent (Variables|Default|GetBP_HealthComponent))
  (:Pressed
    (Default|SetHealth _bp_healthcomponent (+ (Variables|/Game/Blueprints/Entities/EntityComponents/BP_HealthComponent.BP_HealthComponent_C|GetCurr%20Health _bp_healthcomponent) 10))))

(fn ConstructionScript)

(fn InitializeShields
  (bind _base_maxshields (Variables|Shield|GetBase%20MaxShields))
  (Variables|Shield|SetCurr%20Shields _base_maxshields)
  (Variables|Shield|SetCurr%20MaxShields _base_maxshields)
  (Variables|Shield|SetCurr%20ShieldRegen (Variables|Shield|GetBase%20ShieldRegen)))

(fn SetMaxShields
  (params (MaxShields :type Integer))
  (Variables|Shield|SetCurr%20MaxShields MaxShields))

(fn SetShields
  (params (Curr%20Shields :type Integer))
  (|DetermineShieldRegen/Dmg (>= Curr%20Shields (Variables|Shield|GetCurr%20Shields)))
  (bind _output_get (Variables|Shield|SetCurr%20Shields Curr%20Shields))
  (return _output_get))

(fn InitializeDamage
  (Variables|Damage☠️|SetCurr%20Damage (Variables|Damage☠️|GetBase%20Damage))
  (Variables|Damage☠️|SetCurr%20Crit (Variables|Damage☠️|GetBase%20Crit)))

(fn InitializeStats
  (bind _self self)
  (Default|InitializeHealth (Variables|Default|GetBP_HealthComponent))
  (Default|InitializeMovement (Variables|Default|GetBP_MovementStatComponent) _self)
  (Default|InitializeModManager (Variables|Default|GetBP_ModManager) _self))

(fn PrimaryAction
  (if (Variables|Default|GetcanUsePrimary)
    (Default|CallOnUseItem)))

(fn MovementAction
  (Default|CallOnSpecialMovement (Variables|Input|GetInputVector)))