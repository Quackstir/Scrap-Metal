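; Actor component that holds movement stats for an entity and scales its CharacterMovement speed.
; On initialization it caches the entity's CharacterMovement with its starting acceleration, walk speed and braking deceleration, and resets current speed, jump height and jump count to base values.
; ModifyMovement treats the new speed as a multiplier on all three cached values, avoiding compounding changes.
; Jump stats are only stored here, not applied.
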(fn InitializeMovement
  (params (Entity :type BP%20Entity%20Base%20Object%20Reference))
  (bind _output_get (Variables|Default|SetEntity Entity))
  (Variables|Default|SetCharacter%20Movement (Variables|/Script/Engine.Character|GetCharacterMovement _output_get))
  (Variables|Movement|SetCurr%20MovementSpeed (Variables|Movement|GetBase%20MovementSpeed))
  (Variables|Jump|SetCurr%20JumpHeight (Variables|Jump|GetBase%20JumpHeight))
  (Variables|Jump|SetCurr%20JumpAmount (Variables|Jump|GetBase%20JumpAmount))
  (Variables|Default|SetInitial%20Acceleration (Class|CharacterMovementComponent|GetMaxAcceleration (Variables|Default|GetCharacter%20Movement)))
  (Variables|Default|SetInitial%20Walk%20Max%20Speed (Variables|/Script/Engine.CharacterMovementComponent|GetMaxWalkSpeed (Variables|Default|GetCharacter%20Movement)))
  (Variables|Default|SetInitial%20Deceleration (Variables|/Script/Engine.CharacterMovementComponent|GetBrakingDecelerationWalking (Variables|Default|GetCharacter%20Movement))))

(fn ModifyMovement
  (params (New%20MovementSpeed :type Float%20%28double-precision%29))
  (bind _character_movement (Variables|Default|GetCharacter%20Movement))
  (bind _output_get (Variables|Movement|SetCurr%20MovementSpeed New%20MovementSpeed))
  (Variables|/Script/Engine.CharacterMovementComponent|SetMaxAcceleration _character_movement (* _output_get (Variables|Default|GetInitial%20Acceleration)))
  (Variables|/Script/Engine.CharacterMovementComponent|SetMaxWalkSpeed _character_movement (* (Variables|Movement|GetCurr%20MovementSpeed) (Variables|Default|GetInitial%20Walk%20Max%20Speed)))
  (Variables|/Script/Engine.CharacterMovementComponent|SetBrakingDecelerationWalking _character_movement (* (Variables|Movement|GetCurr%20MovementSpeed) (Variables|Default|GetInitial%20Deceleration))))