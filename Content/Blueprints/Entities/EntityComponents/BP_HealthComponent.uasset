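; Health component for entities that stores current and max health, both initialized from a base max value.
; Setting health compares the new value to the old to fire OnHealing (equal or higher) or OnDamage, then stores it unclamped and fires OnModified.
; Max health has its own setter, which fires no events and leaves current health untouched.
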(fn InitializeHealth
  (bind _base_maxhealth (Variables|Default|GetBase%20MaxHealth))
  (Variables|Default|SetCurr%20Health _base_maxhealth)
  (Variables|Default|SetCurr%20MaxHealth _base_maxhealth))

(fn SetHealth
  (params (New%20Health :type Integer))
  (|DetermineHeal/Dmg (>= New%20Health (Variables|Default|GetCurr%20Health)))
  (Variables|Default|SetCurr%20Health New%20Health)
  (Default|CallOnModified))

(fn SetMaxHealth
  (params (Curr%20MaxHealth :type Integer))
  (Variables|Default|SetCurr%20MaxHealth Curr%20MaxHealth))