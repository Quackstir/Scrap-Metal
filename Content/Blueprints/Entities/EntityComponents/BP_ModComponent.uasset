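; BP_ModComponent is an entity component that manages the mods applied to its Entity, which is cached through InitializeModManager.
; AddMod looks the mod struct up in the ModList map and increases the amount on the existing instance when found.
; Otherwise it prints the class name, spawns that class as an actor at the Entity's transform, initializes it with the amount and stores it in the map.
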(fn AddMod
  (params (Amount%20Add :type Integer) (InputPin :type Struct%20Mod%20Structure%20%28by%20ref%29))
  (bind _mod_list (Variables|Default|GetMod%20List))
  (bind (_value _returnvalue) (Utilities|Map|Find _mod_list InputPin))
  (Variables|Default|SetAmount%20Add Amount%20Add)
  (if _returnvalue
    (Default|IncreaseAmount _value (Variables|Default|GetAmount%20Add))
    (else
      (|AddingMod InputPin))))

(fn InitializeModManager
  (params (Entity :type BP%20Entity%20Base%20Object%20Reference))
  (Variables|Default|SetEntity Entity))