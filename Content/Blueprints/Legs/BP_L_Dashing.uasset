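; Dashing legs Blueprint whose special move spends one of up to three dash charges to launch the character.
; A timeline forces high velocity along input, or actor forward without input, with zero braking friction.
; After a short delay it drops speed and sets braking friction to the initially cached GroundFriction.
; A self-restarting regen timeline drives DashRefill and restores charges one at a time, with sound cues.
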(event Custom|Regen%20Dash
  (bind _newtrack_0 (Timeline|TL_DashRegen PlayFromStart)
    (:Update
      (Variables|Default|SetRegeneratingDash true)
      (Variables|Default|SetDashRefill _newtrack_0))
    (:Finished
      (Math|Integer|IncrementInt (Variables|Default|GetDashes)
        (:%20%20
          (if (< (Variables|Default|GetDashes) 3)
            (CallFunction|RegenDash)
            (Audio|PlaySound2D "/Game/StarterContent/Audio/Explosion01.Explosion01" 1.0 1.0 0.0 0 0)
            (else
              (Variables|Default|SetRegeneratingDash false)
              (Audio|PlaySound2D "/Game/StarterContent/Audio/Explosion02.Explosion02" 1.0 1.0 0.0 0 0))))))))

(event EventInitializeVariablesEvent
  (params (Entity :type BP%20Entity%20Base%20Object%20Reference))
  (|CallParentFunction Entity)
  (CallFunction|RegenDash)
  (Variables|Default|SetInitial%20Break%20Friction (Variables|/Script/Engine.CharacterMovementComponent|GetGroundFriction (Variables|Default|GetCharacterMovement))))

(event EventSpecialMove
  (params (Input%20Vector :type Vector :default "0, 0, 0"))
  (bind _charactermovement (Variables|Default|GetCharacterMovement))
  (bind _charactermovement_2 (Variables|Default|GetCharacterMovement))
  (bind _dashes (Variables|Default|GetDashes))
  ;[1 1 1] Dash
  (|CallParentFunction Input%20Vector)
  (if (> _dashes 0)
    (Math|Integer|DecrementInt _dashes
      (:%20%20
        (Variables|Default|SetDashRefill 0.0)
        (Audio|Components|Audio|Play (Variables|Default|GetAudio) 0.0)
        (Timeline|TL_Dashing PlayFromStart
          (:Update
            (Variables|/Script/Engine.MovementComponent|SetVelocity _charactermovement (* (select (Math|Vector|Equal(Vector) (Variables|Default|GetInput%20Vector) "0, 0, 0" 0.2) (Transformation|GetActorForwardVector (Variables|Default|GetEntity)) (Math|Vector|Normalize (Variables|Default|GetInput%20Vector))) 3e+03))
            (Variables|/Script/Engine.CharacterMovementComponent|SetBrakingFriction _charactermovement 0.0))
          (:Finished
            (Utilities|FlowControl|Delay 0.2)
            (Variables|/Script/Engine.MovementComponent|SetVelocity _charactermovement_2 (* (Variables|Default|GetInput%20Vector) 5e+02))
            (Variables|/Script/Engine.CharacterMovementComponent|SetBrakingFriction _charactermovement_2 (Variables|Default|GetInitial%20Break%20Friction))
            (if (not (Variables|Default|GetRegeneratingDash))
              (CallFunction|RegenDash))))))))

(fn ConstructionScript
  (|CallParentFunction))